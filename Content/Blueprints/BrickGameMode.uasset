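; BrickGameMode is the game mode that sets up the brick buildings and saves the world.
; On BeginPlay it starts a new game on every BrickGrid, passes them to the player controller and caches the sky sphere.
; SaveGame writes the first grid, player transform and sky time to the "World" slot.
; Releasing H restarts the second grid found in the level.
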(event EventBeginPlay
  ;[1 1 1] Find the level's BrickGrid
  (bind _outactors (Actor|GetAllActorsOfClass "/Game/Blueprints/BrickGrid.BrickGrid_C"))
  (bind _output_get (Variables|Default|SetBuildings _outactors))
  (CallFunction|InitializationOfBuildings _output_get)
  (Class|BPIHUDInterfaceEvents|InitializacionOfBuildingsCompleted(Message) (Game|GetPlayerController 0) _output_get)
  ;[1 1 1] Find the level's Sky Sphere
  (bind _outactors_2 (Actor|GetAllActorsOfClass "/Game/Sky/BP_BrickSkySphere.BP_BrickSkySphere_C"))
  (Variables|Default|SetSky%20Sphere (Utilities|Array|Get(acopy) _outactors_2)))

(event Input|KeyboardEvents|H
  (:Released
    (bind _outactors (Actor|GetAllActorsOfClass "/Game/Blueprints/BrickGrid.BrickGrid_C"))
    (bind _output_get (Variables|Default|SetHouse (Utilities|Array|Get(acopy) _outactors 1)))
    (Default|NewGame _output_get)))

(fn ConstructionScript)

(fn SaveGame
  (bind _returnvalue (SaveGame|CreateSaveGameObject "/Game/Blueprints/BrickSaveGame.BrickSaveGame_C"))
  (bind _asbrick_save_game (Utilities|Casting|CastToBrickSaveGame _returnvalue))
  (Default|SaveGame (Variables|Default|GetBrick%20Grid) _asbrick_save_game)
  (Variables|/Game/Blueprints/BrickSaveGame.BrickSaveGame_C|SetPlayerTransform _asbrick_save_game (Transformation|GetActorTransform (Game|GetPlayerCharacter 0)))
  (Variables|/Game/Blueprints/BrickSaveGame.BrickSaveGame_C|SetTime%20in%20Days _asbrick_save_game (Default|GetTimeinDays (Variables|Default|GetSky%20Sphere)))
  (SaveGame|SaveGametoSlot _asbrick_save_game "World" (Class|KismetSystemLibrary|MakeLiteralInteger)))

(fn InitializationOfBuildings
  (params (Array :type Array%20of%20Brick%20Grid%20Object%20References))
  (for _array_element Array
    (Default|NewGame _array_element))
  (Variables|Default|SetBrick%20Grid (Utilities|Array|Get(acopy) Array)))